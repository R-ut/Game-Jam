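; EvilDad_BP is a boss enemy that fires an EvilBottle_BP toward the player character on a looping one-second timer.
; ShootBottle takes the last BP_ThirdPersonCharacter found and solves the ballistic equation from Velocity, Gravity, horizontal distance and height difference.
; It spawns the bottle at its own location with look-at yaw and the lower of the two launch angles as pitch.
; If no real solution exists, it prints "Unreachable".
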(event Custom|Bottle
  (CallFunction|ShootBottle))

(event EventBeginPlay
  (Utilities|Time|SetTimerbyEvent (delegate Custom|Bottle) 1.0 true))

(event Collision|EventActorBeginOverlap
  (params (OtherActor :type Actor%20Object%20Reference)))

(fn ConstructionScript)

(fn ShootBottle
  (bind _returnvalue (Transformation|GetActorLocation))
  (bind _returnvalue_2 (Transformation|GetActorLocation))
  (bind _gravity (Variables|Default|GetGravity))
  (bind _velocity (Variables|Default|GetVelocity))
  (bind _returnvalue_3 (Math|Float|Square _velocity))
  (bind _outactors (Actor|GetAllActorsOfClass "/Game/ThirdPerson/Blueprints/BP_ThirdPersonCharacter.BP_ThirdPersonCharacter_C"))
  (for _array_element _outactors
    _)
  (if (>= (- (Math|Float|Square _returnvalue_3) (* (+ (* (Math|Float|Square (Math|Vector2D|Vector2DLength (Math|Vector2D|MakeVector2D (- (.x (Transformation|GetActorLocation _array_element)) (.x _returnvalue_2)) (- (.y (Transformation|GetActorLocation _array_element)) (.y _returnvalue_2))))) _gravity) (* (* (- (.z (Transformation|GetActorLocation _array_element)) (.z _returnvalue_2)) _returnvalue_3) 2.0)) _gravity)) 0.0)
    (Game|SpawnActorfromClass "/Game/EnemyBossAI/EvilBottle_BP.EvilBottle_BP_C" (Math|Transform|MakeTransform _returnvalue (Math|Rotator|MakeRotator (.roll (Math|Rotator|FindLookatRotation _returnvalue (Transformation|GetActorLocation _array_element))) (Math|Float|Min(Float) (Class|KismetMathLibrary|DegAtan (/ (+ (Math|Float|Sqrt (- (Math|Float|Square _returnvalue_3) (* (+ (* (Math|Float|Square (Math|Vector2D|Vector2DLength (Math|Vector2D|MakeVector2D (- (.x (Transformation|GetActorLocation _array_element)) (.x _returnvalue_2)) (- (.y (Transformation|GetActorLocation _array_element)) (.y _returnvalue_2))))) _gravity) (* (* (- (.z (Transformation|GetActorLocation _array_element)) (.z _returnvalue_2)) _returnvalue_3) 2.0)) _gravity))) _returnvalue_3) (* (Math|Vector2D|Vector2DLength (Math|Vector2D|MakeVector2D (- (.x (Transformation|GetActorLocation _array_element)) (.x _returnvalue_2)) (- (.y (Transformation|GetActorLocation _array_element)) (.y _returnvalue_2)))) _gravity))) (Class|KismetMathLibrary|DegAtan (/ (- _returnvalue_3 (Math|Float|Sqrt (- (Math|Float|Square _returnvalue_3) (* (+ (* (Math|Float|Square (Math|Vector2D|Vector2DLength (Math|Vector2D|MakeVector2D (- (.x (Transformation|GetActorLocation _array_element)) (.x _returnvalue_2)) (- (.y (Transformation|GetActorLocation _array_element)) (.y _returnvalue_2))))) _gravity) (* (* (- (.z (Transformation|GetActorLocation _array_element)) (.z _returnvalue_2)) _returnvalue_3) 2.0)) _gravity)))) (* (Math|Vector2D|Vector2DLength (Math|Vector2D|MakeVector2D (- (.x (Transformation|GetActorLocation _array_element)) (.x _returnvalue_2)) (- (.y (Transformation|GetActorLocation _array_element)) (.y _returnvalue_2)))) _gravity)))) (.yaw (Math|Rotator|FindLookatRotation _returnvalue (Transformation|GetActorLocation _array_element)))) "1.000000,1.000000,1.000000") "Undefined" "MultiplyWithRoot" 0 0)
    (else
      (Development|PrintString "Unreachable" true true "(R=1.000000,G=0.000000,B=0.000000,A=1.000000)"))))